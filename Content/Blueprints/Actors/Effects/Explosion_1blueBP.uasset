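; Explosion effect actor built from two material billboards that share a tint taken from a Color variable.
; The construction script gives each billboard a dynamic instance of its own projectile material and sets that instance's color parameter.
; On BeginPlay, a negative actor yaw shifts the second billboard slightly along its local Y axis.
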(event EventBeginPlay
  (if (< (.yaw (Transformation|GetActorRotation)) 0.0)
    (Transformation|AddLocalOffset (Variables|Default|GetMaterialBillboard1) "0,-2.000000, 0" false true)))

(event EventActorBeginOverlap
  (params (OtherActor :type Actor%20Object%20Reference)))

(event EventTick
  (params (DeltaSeconds :type Float%20%28single-precision%29)))

(fn ConstructionScript
  (bind _returnvalue (Rendering|Material|CreateDynamicMaterialInstance (Variables|Default|GetMaterialBillboard) 0 "/Game/Mats/ProjectileMat_1_Inst.ProjectileMat_1_Inst" :!class /Script/Engine.PrimitiveComponent))
  (Rendering|Material|SetVectorParameterValue _returnvalue "color" (Variables|Default|Getcolor) :!class /Script/Engine.MaterialInstanceDynamic)
  (bind _returnvalue_2 (Rendering|Material|CreateDynamicMaterialInstance (Variables|Default|GetMaterialBillboard1) 0 "/Game/Mats/ProjectileMat_2_Inst.ProjectileMat_2_Inst" :!class /Script/Engine.PrimitiveComponent))
  (Rendering|Material|SetVectorParameterValue _returnvalue_2 "color" (Variables|Default|Getcolor) :!class /Script/Engine.MaterialInstanceDynamic))