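; UpDownMoveComp is a component that oscillates its owning actor up and down along its local Z axis.
; It caches the owner at BeginPlay and accumulates elapsed time each Tick to drive a sine wave set by Period and Amplitude.
; The sine value is applied as a swept per-frame offset without delta-time scaling, so travel depends on frame rate and Period acts as a frequency multiplier.
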(event EventBeginPlay
  (Variables|Default|SetMyPawn (Components|GetOwner)))

(event EventTick
  (params (DeltaSeconds :type Float%20%28single-precision%29))
  (bind _output_get (Variables|Default|Settime (+ (Variables|Default|Gettime) DeltaSeconds)))
  (Transformation|AddActorLocalOffset (Variables|Default|GetMyPawn) (Math|Vector|MakeVector 0.0 0.0 (* (Math|Trig|Sin(Radians) (* (Math|Float|MultiplybyPi _output_get) (Variables|Default|GetPeriod))) (Variables|Default|GetAmplitude))) true false))