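; AvoidWallMoveComp is a movement component that keeps its owning Projectile from dropping into surfaces beneath it.
; Each tick it line-traces 100 units straight down on the Camera channel.
; On a hit, it teleports the projectile to hover that distance above the impact and overwrites its ProjectileMovement velocity with a fixed world +Y speed.
; It also accumulates elapsed time, which this graph never reads.
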(event EventBeginPlay
  (bind _asprojectile (Utilities|Casting|CastToProjectile (Components|GetOwner)))
  (Variables|Default|SetMyPawn _asprojectile))

(event EventTick
  (params (DeltaSeconds :type Float%20%28single-precision%29))
  (bind _mypawn (Variables|Default|GetMyPawn))
  (bind _mypawn_2 (Variables|Default|GetMyPawn))
  (bind _returnvalue (Transformation|GetActorLocation _mypawn_2))
  (bind _returnvalue_2 (Transformation|GetActorLocation _mypawn))
  (Variables|Default|Settime (+ (Variables|Default|Gettime) DeltaSeconds))
  (bind (_outhit _returnvalue_3) (Collision|LineTraceByChannel _returnvalue (+ _returnvalue (Math|Vector|MakeVector 0.0 0.0 -1e+02)) "TraceTypeQuery2" false 0 "None"))
  (if _returnvalue_3
    (Transformation|SetActorLocation _mypawn (Math|Vector|MakeVector (.x _returnvalue_2) (.y _returnvalue_2) (+ (.z (.location _outhit)) 1e+02)) false true)
    (Variables|/Script/Engine.MovementComponent|SetVelocity (Variables|/Game/Blueprints/Actors/Projectiles/Projectile.Projectile_C|GetProjectileMovement _mypawn) "0,3000.000000, 0")))