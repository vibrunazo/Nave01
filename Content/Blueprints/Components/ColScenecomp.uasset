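; ColScenecomp is a scene component that gives its owning actor a sphere collision at runtime.
; On BeginPlay or a test event, Inispawn asks ShipGameMode to add the sphere to the owner, unless one is already valid.
; It stores the returned sphere, applies the component's Radius, and prints debug strings along the way.
; Unconnected leftover nodes show earlier attempts that spawned helper actors to create the sphere.
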(event Custom|test
  (CallFunction|Inispawn))

(event EventBeginPlay
  (CallFunction|Inispawn))

(event EventTick
  (params (DeltaSeconds :type Float%20%28single-precision%29)))

(fn Inispawn
  (Utilities|IsValid (Variables|Default|Getsphere)
    (:Is%20Valid
      (Development|PrintString "valid"))
    (:Is%20Not%20Valid
      (bind _asship_game_mode (Utilities|Casting|CastToShipGameMode (Game|GetGameMode))
        (:then
          (bind _sphere (Default|AddSphereCollision _asship_game_mode (Components|GetOwner)))
          (bind _output_get (Variables|Default|Setsphere _sphere))
          (Components|Sphere|SetSphereRadius _output_get (Variables|Default|Getradius) true)
          (Development|PrintString "end"))
        (:CastFailed
          (Development|PrintString "cast fail"))))))