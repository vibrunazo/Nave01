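; Weapon Blueprint that handles firing for a Ship and tracks attack availability through a Canattack flag.
; Fire clears the flag, calls SetCooldown, then passes the Ship to WeaponAttack.
; Two reset routines restore the flag, but the Attackrate-based timers in the Set Cooldown graph are disconnected, so nothing shown triggers a reset.
; The Canattack check in the event graph is also unwired, so Fire runs ungated.
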(event Custom|Fire
  (params (Ship :type Ship%2001%20Object%20Reference))
  (Utilities|FlowControl|Sequence
    (:then_0
      (Variables|Default|Setcanattack false))
    (:then_1
      (|SetCooldown))
    (:then_2
      (CallFunction|WeaponAttack Ship))))

(fn ResetWCooldown
  (Variables|Default|Setcanattack true))

(event Custom|Reset%20Cooldown
  (Variables|Default|Setcanattack true))